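; Game mode for the multiplayer tank game's character selection lobby, from player join to map travel.
; Each joining controller is tracked and given a BP_SelectedCharacter in one of four fixed corner slots, and the game state displays the grid once two players are present.
; StartGame saves tank types by player unique ID in the game instance and opens the map selector.
; LoadMap fades players out and runs ServerTravel.
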(event Custom|StartGame
  (Utilities|Map|Clear (Variables|/Game/GameAssets/Blueprint/GameModes/BP_TankGameInstance.BP_TankGameInstance_C|GetPlayerIDTankType (Variables|Default|GetAs%20BP%20Tank%20Game%20Instance)))
  (for (_array_element _array_index) (Variables|Default|GetAlPlayersPC)
    (Utilities|Map|Add (Variables|/Game/GameAssets/Blueprint/GameModes/BP_TankGameInstance.BP_TankGameInstance_C|GetPlayerIDTankType (Variables|Default|GetAs%20BP%20Tank%20Game%20Instance)) (PlayerState|GetUniqueID (Variables|/Script/Engine.Controller|GetPlayerState _array_element)) (Variables|/Game/GameAssets/Blueprint/UI/Menus/CharacterSelection/BP_SelectedCharacter.BP_SelectedCharacter_C|GetTank%20Type (Utilities|Array|Get(acopy) (Variables|Default|GetPlayersSelectedCharacters) _array_index))))
  (bind _returnvalue (UserInterface|CreateWidget "/Game/GameAssets/Blueprint/UI/Menus/MapSelector/WBP_MapSelector.WBP_MapSelector_C"))
  (UserInterface|Viewport|AddtoViewport _returnvalue 0))

(event Custom|LoadMap
  (params (MapName :type String))
  (for _array_element (Variables|Default|GetAlPlayersPC)
    (bind _asbp_tank_player_controller (Utilities|Casting|CastToBP_TankPlayerController _array_element)
      (:then
        (Default|BlackFadein _asbp_tank_player_controller true))
      (:CastFailed
        (Development|PrintString "Could not cast to BP_TankPlayerController"))))
  (Variables|/Game/GameAssets/Blueprint/GameModes/BP_TankGameInstance.BP_TankGameInstance_C|SetGameStatus (Variables|Default|GetAs%20BP%20Tank%20Game%20Instance) "NewEnumerator1")
  (Development|ExecuteConsoleCommand (Utilities|String|Append "ServerTravel " MapName) 0))

(event EventPostLogin
  (params (NewPlayer :type Player%20Controller%20Object%20Reference)))

(event EventOnLogout
  (params (ExitingController :type Controller%20Object%20Reference))
  (bind _asplayer_controller (Utilities|Casting|CastToPlayerController ExitingController))
  (Utilities|Array|RemoveItem (Variables|Default|GetAlPlayersPC) _asplayer_controller))

(event EventBeginPlay
  (bind _asbp_tank_game_instance (Utilities|Casting|CastToBP_TankGameInstance (Game|GetGameInstance))
    (:then
      (Variables|Default|SetAs%20BP%20Tank%20Game%20Instance _asbp_tank_game_instance))
    (:CastFailed
      (Development|PrintString "Could not get custom game instance"))))

(event EventHandleStartingNewPlayer
  (params (NewPlayer :type Player%20Controller%20Object%20Reference))
  (bind _asbp_tank_player_controller (Utilities|Casting|CastToBP_TankPlayerController NewPlayer)
    (:then
      (Default|BlackFadeOut _asbp_tank_player_controller true)
      (Utilities|Array|AddUnique (Variables|Default|GetAlPlayersPC) NewPlayer)
      (Development|PrintString (Utilities|String|Append "A new player has joined : " (Utilities|GetDisplayName NewPlayer)))
      ;[0.15 0.15 0.15 0.5] Spawn for character selection
      (CallFunction|SpawnActor NewPlayer)
      ;[0.15 0.15 0.15 0.5] Display Grid via game State
      (if (> (Utilities|Array|Length (Variables|Default|GetAlPlayersPC)) 1)
        (CallFunction|GetGameState)
        (Default|DisplayGrid (Variables|Default|GetAs%20BP%20Selection%20Charactergame%20State))))
    (:CastFailed
      (Development|PrintString "Could not cast to BP_TankPlayerController"))))

(fn ConstructionScript)

(fn SpawnActor
  (params (PlayerController :type Player%20Controller%20Object%20Reference))
  (if (== 1 (Utilities|Array|Length (Variables|Default|GetAlPlayersPC)))
    ;[0.15 0.15 0.15 0.5] Top Left
    (bind _returnvalue (Game|SpawnActorfromClass "/Game/GameAssets/Blueprint/UI/Menus/CharacterSelection/BP_SelectedCharacter.BP_SelectedCharacter_C" (Math|Transform|MakeTransform "1180.000000,-520.000000,720.000000") "AlwaysSpawn" "MultiplyWithRoot" PlayerController 0))
    (Utilities|Array|AddUnique (Variables|Default|GetPlayersSelectedCharacters) _returnvalue)
    (elif (== 2 (Utilities|Array|Length (Variables|Default|GetAlPlayersPC)))
      ;[0.15 0.15 0.15 0.5] Top Right
      (bind _returnvalue_2 (Game|SpawnActorfromClass "/Game/GameAssets/Blueprint/UI/Menus/CharacterSelection/BP_SelectedCharacter.BP_SelectedCharacter_C" (Math|Transform|MakeTransform "1180.000000,520.000000,720.000000" "0.000000,60.000000,0.000000") "AlwaysSpawn" "MultiplyWithRoot" PlayerController 0))
      (Utilities|Array|AddUnique (Variables|Default|GetPlayersSelectedCharacters) _returnvalue_2)
      (elif (== 3 (Utilities|Array|Length (Variables|Default|GetAlPlayersPC)))
        ;[0.15 0.15 0.15 0.5] Bottom Left
        (bind _returnvalue_3 (Game|SpawnActorfromClass "/Game/GameAssets/Blueprint/UI/Menus/CharacterSelection/BP_SelectedCharacter.BP_SelectedCharacter_C" (Math|Transform|MakeTransform "1100.000000,-520.000000,310.000000" "-25.000000,0.000000,0.000000") "AlwaysSpawn" "MultiplyWithRoot" PlayerController 0))
        (Utilities|Array|AddUnique (Variables|Default|GetPlayersSelectedCharacters) _returnvalue_3)
        (elif (== 4 (Utilities|Array|Length (Variables|Default|GetAlPlayersPC)))
          ;[0.15 0.15 0.15 0.5] Bttom Right
          (bind _returnvalue_4 (Game|SpawnActorfromClass "/Game/GameAssets/Blueprint/UI/Menus/CharacterSelection/BP_SelectedCharacter.BP_SelectedCharacter_C" (Math|Transform|MakeTransform "1100.000000,520.000000,310.000000" "-15.000000,60.000000,-25.000000") "AlwaysSpawn" "MultiplyWithRoot" PlayerController 0))
          (Utilities|Array|AddUnique (Variables|Default|GetPlayersSelectedCharacters) _returnvalue_4))))))

(fn GetWidgets
  ;[0.15 0.15 0.15 0.5] Widget Background
  (bind _returnvalue (Actor|GetActorOfClass "/Game/GameAssets/Blueprint/UI/Menus/CharacterSelection/BP_CharacterSelectionActor.BP_CharacterSelectionActor_C"))
  (Development|PrintString (Utilities|GetDisplayName _returnvalue) true true "(R=1.000000,G=0.508637,B=0.000000,A=1.000000)")
  (bind _aswbp_background (Utilities|Casting|CastToWBP_Background (UserInterface|GetUserWidgetObject (Variables|/Game/GameAssets/Blueprint/UI/Menus/CharacterSelection/BP_CharacterSelectionActor.BP_CharacterSelectionActor_C|GetWidget _returnvalue)))
    (:then
      (Variables|Default|SetAs%20WBP%20Background _aswbp_background)
      ;[0.15 0.15 0.15 0.5] Widget Character Selection
      (bind _foundwidgets (Widget|GetAllWidgetsOfClass "/Game/GameAssets/Blueprint/UI/Menus/CharacterSelection/WBP_CharacterSelection.WBP_CharacterSelection_C" false))
      (bind _output_get (Variables|Default|SetAs%20WBP%20Character%20Selection (Utilities|Array|Get(acopy) _foundwidgets)))
      (Utilities|IsValid _output_get
        (:Is%20Not%20Valid
          (Development|PrintString "Invalid Widget"))))
    (:CastFailed
      (Development|PrintString "cast  failed"))))

(fn ShowCharactersGrid
  (if (> (Utilities|Array|Length (Variables|Default|GetAlPlayersPC)) 1)
    (for _array_element (Variables|Default|GetAlPlayersPC)
      ;[0.15 0.15 0.15 0.5] Hide waiting text
      (Widget|SetVisibility (Variables|/Game/GameAssets/Blueprint/UI/Menus/CharacterSelection/WBP_Background.WBP_Background_C|GetTXT_Wait (Variables|Default|GetAs%20WBP%20Background)) "Hidden")
      ;[0.15 0.15 0.15 0.5] Show Chracters Grid
      (Widget|SetVisibility (Variables|/Game/GameAssets/Blueprint/UI/Menus/CharacterSelection/WBP_CharacterSelection.WBP_CharacterSelection_C|GetGrid_Images (Variables|Default|GetAs%20WBP%20Character%20Selection)) "Visible"))))

(fn GetGameState
  (Utilities|IsValid (Variables|Default|GetAs%20BP%20Selection%20Charactergame%20State)
    (:Is%20Not%20Valid
      (bind _asbp_selection_character_game_state (Utilities|Casting|CastToBP_SelectionCharacterGameState (Game|GetGameState))
        (:then
          (Variables|Default|SetAs%20BP%20Selection%20Charactergame%20State _asbp_selection_character_game_state))
        (:CastFailed
          (Development|PrintString "game state cast failed"))))))