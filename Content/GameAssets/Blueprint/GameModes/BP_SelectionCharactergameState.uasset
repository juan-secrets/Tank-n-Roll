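; Game state for the character selection screen that creates the selection widget and triggers filling of its grid.
; BeginPlay adds WBP_CharacterSelection to the first player's viewport and caches it.
; DisplayGrid sets a RepNotify toggle whose OnRep calls FillGrid on that widget, so replication drives the grid display.
; GetWidgets, not called within this graph, caches the background widget from BP_CharacterSelectionActor and looks up the selection widget, printing debug messages.
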(event Custom|DisplayGrid
  (Variables|Default|SetDisplayGridToggle true))

(event EventBeginPlay
  (bind _returnvalue (UserInterface|CreateWidget "/Game/GameAssets/Blueprint/UI/Menus/CharacterSelection/WBP_CharacterSelection.WBP_CharacterSelection_C" (Game|GetPlayerController 0)))
  (UserInterface|Viewport|AddtoViewport _returnvalue 0)
  (Variables|Default|SetAs%20WBP%20Character%20Selection _returnvalue))

(fn ConstructionScript)

(fn GetWidgets
  ;[0.15 0.15 0.15 0.5] Widget Background
  (bind _returnvalue (Actor|GetActorOfClass "/Game/GameAssets/Blueprint/UI/Menus/CharacterSelection/BP_CharacterSelectionActor.BP_CharacterSelectionActor_C"))
  (Development|PrintString (Utilities|GetDisplayName _returnvalue) true true "(R=1.000000,G=0.508637,B=0.000000,A=1.000000)")
  (bind _aswbp_background (Utilities|Casting|CastToWBP_Background (UserInterface|GetUserWidgetObject (Variables|/Game/GameAssets/Blueprint/UI/Menus/CharacterSelection/BP_CharacterSelectionActor.BP_CharacterSelectionActor_C|GetWidget _returnvalue)))
    (:then
      (Variables|Default|SetAs%20WBP%20Background _aswbp_background)
      ;[0.15 0.15 0.15 0.5] Widget Character Selection
      (bind _foundwidgets (Widget|GetAllWidgetsOfClass "/Game/GameAssets/Blueprint/UI/Menus/CharacterSelection/WBP_CharacterSelection.WBP_CharacterSelection_C" false))
      (bind _output_get (Variables|Default|SetAs%20WBP%20Character%20Selection (Utilities|Array|Get(acopy) _foundwidgets)))
      (Utilities|IsValid _output_get
        (:Is%20Not%20Valid
          (Development|PrintString "Invalid grid Widget" true true "(R=0.000000,G=0.660000,B=1.000000,A=1.000000)" 999.0))))
    (:CastFailed
      (Development|PrintString "Acotr widget cast  failed" true true "(R=0.000000,G=0.660000,B=1.000000,A=1.000000)" 999.0))))

(fn OnRepDisplayGridToggle
  (Default|FillGrid (Variables|Default|GetAs%20WBP%20Character%20Selection)))