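; Game mode for multiplayer tank matches, handling player login, spawning, win/loss, restart and return to menu.
; It admits players listed in the game instance's tank-choice map and starts once all arrive; debug mode spawns immediately.
; Each player gets their chosen tank at an unowned PlayerStart, which the tank then owns.
; Deaths are tallied until one survivor remains; restart respawns tanks, or travels to CharacterSelection without multiple players.
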(event Custom|StartGame
  ;[0.15 0.15 0.15 0.5] Debug Start Game, we should spawn each tank individually depending on the tank type the player choose
  (CallFunction|SpawnPlayers) ; To remove when new tank types are created
)

(event Custom|SpawnPlayers
  ;[0.15 0.15 0.15 0.5] Player Spawn
  (for _array_element (Variables|Default|GetAlPlayersPC)
    (CallFunction|SpawnPlayer _array_element)))

(event Custom|AllPlayersFadeIn
  (for _array_element (Variables|Default|GetAlPlayersPC)
    (bind _asbp_tank_player_controller (Utilities|Casting|CastToBP_TankPlayerController _array_element)
      (:then
        (Default|BlackFadein _asbp_tank_player_controller true))
      (:CastFailed
        (Development|PrintString "Could not cast to BP_TankPlayerController")))))

(event Custom|SpawnPlayer
  (params (PlayerController :type Player%20Controller%20Object%20Reference))
  ;[0.15 0.15 0.15 0.5] Player Spawn
  (bind _outactors (Actor|GetAllActorsOfClass "/Script/Engine.PlayerStart"))
  (bind _array_element (Utilities|Array|ForEachLoopwithBreak _outactors :!label _label)
    (:LoopBody
      (Utilities|IsValid (Components|GetOwner _array_element)
        (:Is%20Not%20Valid
          (bind _tanktype (CallFunction|GetTankTypebyPlayerController PlayerController))
          (bind _tankclass (CallFunction|GetTankClass _tanktype))
          (bind _returnvalue (Game|SpawnActorfromClass _tankclass (Transformation|GetActorTransform _array_element) "Undefined" "MultiplyWithRoot" 0 0))
          (Actor|SetOwner _array_element _returnvalue)
          (bind _aspawn (Utilities|Casting|CastToPawn _returnvalue)
            (:then
              (Pawn|Possess PlayerController _aspawn)
              (goto _label Break))
            (:CastFailed
              (Development|PrintString "Couldn not cast tank actor to pawn"))))))))

(event Custom|PlayerDied
  (params (PlayerController :type Player%20Controller%20Object%20Reference))
  ;[0.15 0.15 0.15 0.5] Player died event handling
  (Utilities|Map|Add (Variables|Default|GetPlayersDeadStatus) PlayerController true)
  ;;[0.15 0.15 0.15 0.5] Check for only one player left alive
  (if (>= (Utilities|Map|Length (Variables|Default|GetPlayersDeadStatus)) (- (Utilities|Array|Length (Variables|Default|GetAlPlayersPC)) 1))
    (for _array_element (Variables|Default|GetAlPlayersPC)
      (if (not (.ReturnValue (Utilities|Map|Find (Variables|Default|GetPlayersDeadStatus) _array_element)))
        (bind _asbp_player (Utilities|Casting|CastToBP_Player (Pawn|GetControlledPawn _array_element))
          (:then
            (Default|WonGame _asbp_player))
          (:CastFailed
            (Development|PrintString "cast failed for the player that won" :!label _label)))
        (else
          (bind _asbp_player_2 (Utilities|Casting|CastToBP_Player (Pawn|GetControlledPawn _array_element))
            (:then
              (Default|LostGame _asbp_player_2))
            (:CastFailed
              (goto _label))))))))

(event Custom|RestartGame
  ;[0.15 0.15 0.15 0.5] Debug Start Game, we should spawn each tank individually depending on the tank type the player choose
  (Utilities|Map|Clear (Variables|Default|GetPlayersDeadStatus))
  (if (> (Utilities|Array|Length (Variables|Default|GetAlPlayersPC)) 1)
    (for _array_element (Variables|Default|GetAlPlayersPC)
      (bind _asbp_player (Utilities|Casting|CastToBP_Player (Pawn|GetControlledPawn _array_element)))
      (Default|Destroy _asbp_player))
    (CallFunction|AllPlayersFadeOut)
    (Utilities|FlowControl|Delay 1.0)
    (CallFunction|StartGame)
    (else
      (Development|ExecuteConsoleCommand "ServerTravel CharacterSelection" 0))))

(event Custom|MainMenu
  ;[0.15 0.15 0.15 0.5] Make all players go to main menu
  (for _array_element (Variables|Default|GetAlPlayersPC)
    (Utilities|IsValid _array_element
      (:Is%20Valid
        (bind _asbp_tank_player_controller (Utilities|Casting|CastToBP_TankPlayerController _array_element)
          (:then
            (Default|BlackFadein _asbp_tank_player_controller true)
            (Utilities|FlowControl|Delay 0.5)
            (bind _asbp_player (Utilities|Casting|CastToBP_Player (Pawn|GetControlledPawn _array_element)))
            (|DestroySession _array_element
              (:OnSuccess
                _)
              (:OnFailure
                _))
            (Default|MainMenu _asbp_player))
          (:CastFailed
            (Development|PrintString "Could not cast to BP_TankPlayerController"))))))
  (Utilities|FlowControl|Delay 1.0)
  (Utilities|FlowControl|DoOnce false
    (:Completed
      (CallFunction|MainMenu))))

(event Custom|AllPlayersFadeOut
  (for _array_element (Variables|Default|GetAlPlayersPC)
    (bind _asbp_tank_player_controller (Utilities|Casting|CastToBP_TankPlayerController _array_element)
      (:then
        (Default|ClearFadein _asbp_tank_player_controller)
        (Default|BlackFadeOut _asbp_tank_player_controller true))
      (:CastFailed
        (Development|PrintString "Could not cast to BP_TankPlayerController")))))

(event EventPostLogin
  (params (NewPlayer :type Player%20Controller%20Object%20Reference))
  (Development|PrintString "PostLogin Event play of BP_GameplayMode" true true "(R=0.000000,G=0.660000,B=1.000000,A=1.000000)" 6e+01))

(event EventOnLogout
  (params (ExitingController :type Controller%20Object%20Reference))
  (bind _asplayer_controller (Utilities|Casting|CastToPlayerController ExitingController))
  (Utilities|Array|RemoveItem (Variables|Default|GetAlPlayersPC) _asplayer_controller))

(event EventBeginPlay
  (Development|PrintString "Begin play of BP_GameplayMode" true true "(R=0.000000,G=0.660000,B=1.000000,A=1.000000)" 6e+01)
  (CallFunction|GetGameInstance))

(event EventHandleStartingNewPlayer
  (params (NewPlayer :type Player%20Controller%20Object%20Reference))
  (Development|PrintString "Event handle starting new player of BP_GameplayMode" true true "(R=0.000000,G=0.660000,B=1.000000,A=1.000000)" 6e+01)
  (CallFunction|GetGameInstance)
  (CallFunction|HandlePlayerLogin NewPlayer)
  (bind _asbp_tank_player_controller (Utilities|Casting|CastToBP_TankPlayerController NewPlayer)
    (:then
      (Default|BlackFadeOut _asbp_tank_player_controller true))
    (:CastFailed
      (Development|PrintString "Could not cast to BP_TankPlayerController"))))

(fn ConstructionScript)

(fn GetGameInstance
  (Utilities|IsValid (Variables|Default|GetAs%20BP%20Tank%20Game%20Instance)
    (:Is%20Valid
      _)
    (:Is%20Not%20Valid
      (bind _asbp_tank_game_instance (Utilities|Casting|CastToBP_TankGameInstance (Game|GetGameInstance))
        (:then
          (bind _output_get (Variables|Default|SetAs%20BP%20Tank%20Game%20Instance _asbp_tank_game_instance))
          (if (Utilities|Enum|NotEqual(Enum) (Variables|/Game/GameAssets/Blueprint/GameModes/BP_TankGameInstance.BP_TankGameInstance_C|GetGameStatus _output_get) "NewEnumerator1")
            (Variables|Default|SetDebug true)))
        (:CastFailed
          (Development|PrintString "Could not get custom game instance")))))
  (return (Variables|Default|GetAs%20BP%20Tank%20Game%20Instance)))

(fn ShouldStartGame
  (return (>= (Utilities|Array|Length (Variables|Default|GetAlPlayersPC)) (Utilities|Map|Length (Variables|/Game/GameAssets/Blueprint/GameModes/BP_TankGameInstance.BP_TankGameInstance_C|GetPlayerIDTankType (Variables|Default|GetAs%20BP%20Tank%20Game%20Instance))))))

(fn GetPlayerwithUniqueNetID
  (params (ID :type Unique%20Net%20Id%20Repl%20Structure))
  (for (_array_element _array_index) (Variables|Default|GetAlPlayersPC)
    (if (!= (Utilities|Array|FindItem (Utilities|Array|MakeArray ID) (PlayerState|GetUniqueID (Variables|/Script/Engine.Controller|GetPlayerState _array_element))) -1)
      (return _array_element _array_index)))
  (return 0 -1))

(fn HandlePlayerLogin
  (params (PlayerController :type Player%20Controller%20Object%20Reference))
  (if (Variables|Default|GetDebug)
    ;[0.15 0.15 0.15 0.5] Debug for when playing map in editor
    (CallFunction|SpawnPlayer PlayerController)
    (Utilities|Array|AddUnique (Variables|Default|GetAlPlayersPC) PlayerController)
    (elif (not (.ReturnValue (Utilities|Map|Find (Variables|/Game/GameAssets/Blueprint/GameModes/BP_TankGameInstance.BP_TankGameInstance_C|GetPlayerIDTankType (Variables|Default|GetAs%20BP%20Tank%20Game%20Instance)) (PlayerState|GetUniqueID (Variables|/Script/Engine.Controller|GetPlayerState PlayerController)))))
      ;[0.15 0.15 0.15 0.5] If Unknown player join mid game, make it quit
      (Development|PrintString "unknown player ID joined")
      (Game|QuitGame PlayerController "Quit" true)
      (else
        (Utilities|Array|AddUnique (Variables|Default|GetAlPlayersPC) PlayerController)
        (bind _bool (CallFunction|ShouldStartGame))
        (if _bool
          (CallFunction|StartGame))))))

(fn GetTankClass
  (params (TankType :type E_TankType%20Enum :default "NewEnumerator0"))
  (switch Utilities|FlowControl|Switch|SwitchonE_TankType TankType
    (:NewEnumerator0
      (return "/Game/GameAssets/Blueprint/Player/BP_BlueTank1.BP_BlueTank1_C"))
    (:NewEnumerator1
      (return "/Game/GameAssets/Blueprint/Player/BP_BlueTank2.BP_BlueTank2_C"))
    (:NewEnumerator2
      (return "/Game/GameAssets/Blueprint/Player/BP_BlueTank3.BP_BlueTank3_C"))
    (:NewEnumerator3
      (return "/Game/GameAssets/Blueprint/Player/BP_YellowTank1.BP_YellowTank1_C"))
    (:NewEnumerator4
      (return "/Game/GameAssets/Blueprint/Player/BP_YellowTank2.BP_YellowTank2_C"))
    (:NewEnumerator5
      (return "/Game/GameAssets/Blueprint/Player/BP_YellowTank3.BP_YellowTank3_C"))
    (:NewEnumerator6
      (return "/Game/GameAssets/Blueprint/Player/BP_GreenTank1.BP_GreenTank1_C"))
    (:NewEnumerator7
      (return "/Game/GameAssets/Blueprint/Player/BP_GreenTank2.BP_GreenTank2_C"))
    (:NewEnumerator8
      (return "/Game/GameAssets/Blueprint/Player/BP_GreenTank3.BP_GreenTank3_C"))
    (:NewEnumerator9
      (return "/Game/GameAssets/Blueprint/Player/BP_WhiteTank1.BP_WhiteTank1_C"))
    (:NewEnumerator10
      (return "/Game/GameAssets/Blueprint/Player/BP_WhiteTank2.BP_WhiteTank2_C"))
    (:NewEnumerator11
      (return "/Game/GameAssets/Blueprint/Player/BP_WhiteTank3.BP_WhiteTank3_C"))))

(fn GetTankTypebyPlayerController
  (params (PlayerController :type Player%20Controller%20Object%20Reference))
  (bind _asbp_tank_game_instance (Utilities|Casting|CastToBP_TankGameInstance (Game|GetGameInstance))
    (:then
      (if (.ReturnValue (Utilities|Map|Find (Variables|/Game/GameAssets/Blueprint/GameModes/BP_TankGameInstance.BP_TankGameInstance_C|GetPlayerIDTankType _asbp_tank_game_instance) (PlayerState|GetUniqueID (Variables|/Script/Engine.Controller|GetPlayerState PlayerController))))
        (return (.Value (Utilities|Map|Find (Variables|/Game/GameAssets/Blueprint/GameModes/BP_TankGameInstance.BP_TankGameInstance_C|GetPlayerIDTankType _asbp_tank_game_instance) (PlayerState|GetUniqueID (Variables|/Script/Engine.Controller|GetPlayerState PlayerController)))))
        (else
          (Development|PrintString "Could not find the corresponding tank choice")
          (return "NewEnumerator0"))))
    (:CastFailed
      (Development|PrintString "cast to tank game instance failed"))))