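; BP_Shell is a bouncing tank shell projectile that kills players it touches.
; Each ProjectileMovement bounce plays a random sound and spark effect, and the third bounce destroys the shell.
; A hit against another BP_Shell destroys both shells.
; Overlapping a living BP_Player marks it dead, disables its movement, fades out its engine audio, spawns randomized explosion effects and destroys the shell.
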(event OnComponentHit(ShellMesh)
  (params (HitComponent :type Primitive%20Component%20Object%20Reference) (OtherActor :type Actor%20Object%20Reference) (OtherComp :type Primitive%20Component%20Object%20Reference) (NormalImpulse :type Vector :default "0, 0, 0") (Hit :type Hit%20Result%20Structure%20%28by%20ref%29))
  ;[0.15 0.15 0.15 0.5] Detect Shell Hit
  (Utilities|FlowControl|Sequence
    (:then_0
      (Class|KismetSystemLibrary|IsObjectOfSoftClass OtherActor "/Game/GameAssets/Blueprint/Props/BP_Shell.BP_Shell_C"
        (:True
          (Niagara|SpawnSystematLocation "/Game/MixedVFX/Particles/Slashes/SeparateParts/Hits/NS_FireSlash_Hit.NS_FireSlash_Hit" (Transformation|GetActorLocation) "0, 0, 0" "0.300000,0.300000,0.300000")
          (Audio|PlaySoundatLocation "/Game/GameAssets/Assets/SFX/TankDeath.TankDeath" (Transformation|GetActorLocation OtherActor) "0, 0, 0" 0.1 (Math|Random|RandomFloatinRange 0.9 1.1) 0.0 "/Game/GameAssets/Assets/SFX/SA_Shell.SA_Shell" 0 0 0)
          (Actor|DestroyActor OtherActor)
          (Actor|DestroyActor))))))

(event OnComponentBeginOverlap(ShellMesh)
  (params (OverlappedComponent :type Primitive%20Component%20Object%20Reference) (OtherActor :type Actor%20Object%20Reference) (OtherComp :type Primitive%20Component%20Object%20Reference) (OtherBodyIndex :type Integer) (bFromSweep :type Boolean) (SweepResult :type Hit%20Result%20Structure%20%28by%20ref%29))
  (bind _returnvalue (Math|Random|RandomFloatinRange 0.8 1.2))
  ;[0.15 0.15 0.15 0.5] Detect Player Hit
  (Class|KismetSystemLibrary|IsObjectOfSoftClass OtherActor "/Game/GameAssets/Blueprint/Player/BP_Player.BP_Player_C"
    (:True
      (bind _asbp_player (Utilities|Casting|CastToBP_Player OtherActor))
      (if (not (Variables|/Game/GameAssets/Blueprint/Player/BP_Player.BP_Player_C|GetIsDead _asbp_player))
        (Variables|/Game/GameAssets/Blueprint/Player/BP_Player.BP_Player_C|SetIsDead _asbp_player true)
        (Pawn|Components|CharacterMovement|DisableMovement (Variables|/Script/Engine.Character|GetCharacterMovement _asbp_player))
        (Audio|PlaySoundatLocation "/Game/GameAssets/Assets/SFX/TankDeath.TankDeath" (Transformation|GetActorLocation) "0, 0, 0" 0.1 (Math|Random|RandomFloatinRange 0.9 1.1) 0.0 "/Game/GameAssets/Assets/SFX/SA_Shell.SA_Shell" 0 0 0)
        (Audio|Components|Audio|FadeOut (Variables|/Game/GameAssets/Blueprint/Player/BP_Player.BP_Player_C|GetTankEngine _asbp_player) 0.5 0.0 "Linear" :!class /Script/Engine.AudioComponent)
        (Niagara|SpawnSystematLocation "/Game/MixedVFX/Particles/Explosions/NS_ExplosionGroundSmall.NS_ExplosionGroundSmall" (Transformation|GetActorLocation _asbp_player) (Math|Random|RandomRotator true) (Math|Vector|MakeVector _returnvalue _returnvalue _returnvalue))
        (Niagara|SpawnSystematLocation "/Game/MixedVFX/Particles/Mix/NS_Mix_02.NS_Mix_02" (Transformation|GetActorLocation _asbp_player) "0, 0, 0" (Math|Vector|MakeVector _returnvalue _returnvalue _returnvalue))
        (Actor|DestroyActor)))))

(event OnProjectileBounce(ProjectileMovement)
  (params (ImpactResult :type Hit%20Result%20Structure%20%28by%20ref%29) (ImpactVelocity :type Vector%20%28by%20ref%29 :default "0, 0, 0"))
  (bind _returnvalue (Transformation|GetActorLocation))
  ;[0.15 0.15 0.15 0.5] Destroy Shell on its 3rd bounce
  (Audio|PlaySoundatLocation (.OutItem (Utilities|Array|Random (Variables|Default|GetBounceSounds))) _returnvalue "0, 0, 0" 0.1 (Math|Random|RandomFloatinRange 0.9 1.1) 0.0 "/Game/GameAssets/Assets/SFX/SA_Shell.SA_Shell" 0 0 0)
  (Niagara|SpawnSystematLocation "/Game/MixedVFX/Particles/Projectiles/Hits/NS_FireArrow_Hit.NS_FireArrow_Hit" _returnvalue "0, 0, 0" "1.500000,1.500000,1.500000")
  (bind _result (Math|Integer|IncrementInt (Variables|Default|GetProjectileBounces))
    (:%20%20
      (if (> _result 2)
        (Niagara|SpawnSystematLocation "/Game/MixedVFX/Particles/Slashes/SeparateParts/Hits/NS_FireSlash_Hit.NS_FireSlash_Hit" (Transformation|GetActorLocation) "0, 0, 0" "0.300000,0.300000,0.300000")
        (Variables|Default|SetProjectileBounces 0)
        (Audio|PlaySoundatLocation "/Game/GameAssets/Assets/SFX/TankDeath.TankDeath" (Transformation|GetActorLocation) "0, 0, 0" 0.1 (Math|Random|RandomFloatinRange 0.9 1.1) 0.0 "/Game/GameAssets/Assets/SFX/SA_Shell.SA_Shell" 0 0 0)
        (Actor|DestroyActor)))))

(event EventBeginPlay
  (Variables|Default|SetProjectileBounces 0))

(fn ConstructionScript)