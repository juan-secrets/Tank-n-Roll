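; Mortar shell projectile that explodes on its first bounce and instantly kills player tanks within the blast radius.
; On bounce, a sphere overlap for pawns finds each living BP_Player, marks it dead, disables its movement and fades out its engine audio.
; Each kill spawns randomly scaled explosion effects and a pitch-varied death sound.
; The shell always plays its own ground explosion and sound, then destroys itself.
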(event OnProjectileBounce(ProjectileMovement)
  (params (ImpactResult :type Hit%20Result%20Structure%20%28by%20ref%29) (ImpactVelocity :type Vector%20%28by%20ref%29 :default "0, 0, 0"))
  (bind _returnvalue (Math|Random|RandomFloatinRange 0.8 1.2))
  ;[0.15 0.15 0.15 0.5] Detect Shell Hit
  (bind _outactors (Collision|SphereOverlapActors (.ImpactPoint (Collision|BreakHitResult ImpactResult)) 3e+02 (Utilities|Array|MakeArray "ObjectTypeQuery3") 0))
  (for _array_element _outactors
    (Class|KismetSystemLibrary|IsObjectOfSoftClass _array_element "/Game/GameAssets/Blueprint/Player/BP_Player.BP_Player_C"
      (:True
        (bind _asbp_player (Utilities|Casting|CastToBP_Player _array_element))
        (if (not (Variables|/Game/GameAssets/Blueprint/Player/BP_Player.BP_Player_C|GetIsDead _asbp_player))
          (Variables|/Game/GameAssets/Blueprint/Player/BP_Player.BP_Player_C|SetIsDead _asbp_player true)
          (Pawn|Components|CharacterMovement|DisableMovement (Variables|/Script/Engine.Character|GetCharacterMovement _asbp_player))
          ;;[0.15 0.15 0.15 0.5] Player Death VFX/SFX
          (Audio|PlaySoundatLocation "/Game/GameAssets/Assets/SFX/TankDeath.TankDeath" (Transformation|GetActorLocation) "0, 0, 0" 0.1 (Math|Random|RandomFloatinRange 0.9 1.1) 0.0 "/Game/GameAssets/Assets/SFX/SA_Shell.SA_Shell" 0 0 0)
          (Audio|Components|Audio|FadeOut (Variables|/Game/GameAssets/Blueprint/Player/BP_Player.BP_Player_C|GetTankEngine _asbp_player) 0.5 0.0 "Linear" :!class /Script/Engine.AudioComponent)
          (Niagara|SpawnSystematLocation "/Game/MixedVFX/Particles/Explosions/NS_ExplosionGroundSmall.NS_ExplosionGroundSmall" (Transformation|GetActorLocation _asbp_player) (Math|Random|RandomRotator true) (Math|Vector|MakeVector _returnvalue _returnvalue _returnvalue))
          (Niagara|SpawnSystematLocation "/Game/MixedVFX/Particles/Mix/NS_Mix_02.NS_Mix_02" (Transformation|GetActorLocation _asbp_player) "0, 0, 0" (Math|Vector|MakeVector _returnvalue _returnvalue _returnvalue))))))
  (Niagara|SpawnSystematLocation "/Game/MixedVFX/Particles/Explosions/NS_ExplosionGroundBig.NS_ExplosionGroundBig" (Transformation|GetActorLocation) "0, 0, 0" "0.500000,0.500000,0.500000")
  (Audio|PlaySoundatLocation "/Game/GameAssets/Assets/SFX/TankDeath.TankDeath" (Transformation|GetActorLocation) "0, 0, 0" 0.1 (Math|Random|RandomFloatinRange 0.9 1.1) 0.0 "/Game/GameAssets/Assets/SFX/SA_Shell.SA_Shell" 0 0 0)
  (Actor|DestroyActor))

(fn ConstructionScript)