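; BP_Bomb is a landmine prop that arms shortly after its owner leaves the trigger, then explodes on overlap or when its fuse runs out.
; Chained delays speed up a looping timer that flip-flops the arming light alongside a beeping sound, ending in a timed detonation.
; MineExplosion kills nearby living BP_Players, posts Steam-name killfeed entries through BP_InGameGameState, plays effects and destroys the actor.
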(event OnComponentBeginOverlap(landmine)
  (params (OverlappedComponent :type Primitive%20Component%20Object%20Reference) (OtherActor :type Actor%20Object%20Reference) (OtherComp :type Primitive%20Component%20Object%20Reference) (OtherBodyIndex :type Integer) (bFromSweep :type Boolean) (SweepResult :type Hit%20Result%20Structure%20%28by%20ref%29))
  ;[0.15 0.15 0.15 0.5] Call Explosion Logic
  (if (Variables|Default|GetIsActivated)
    (CallFunction|MineExplosion)))

(event OnComponentEndOverlap(landmine)
  (params (OverlappedComponent :type Primitive%20Component%20Object%20Reference) (OtherActor :type Actor%20Object%20Reference) (OtherComp :type Primitive%20Component%20Object%20Reference) (OtherBodyIndex :type Integer))
  ;[0.15 0.15 0.15 0.5] Arming Logic
  (if (== OtherActor (Components|GetOwner))
    (Utilities|FlowControl|Delay 1.0)
    (Rendering|SetVisibility (Variables|Default|GetArming%20Light) true false)
    (Variables|Default|SetIsActivated true)
    (bind _returnvalue (Audio|SpawnSoundAttached "/Game/GameAssets/Assets/SFX/BombBeeping.BombBeeping" (Variables|Default|GetDefaultSceneRoot) "None" (Transformation|GetActorLocation) "0, 0, 0" "SnapToTarget" true 0.1 1.0 0.0 "/Game/GameAssets/Assets/SFX/SA_Bomb.SA_Bomb" 0 false))
    (Variables|Default|SetBeepingSFX _returnvalue)
    (CallFunction|SetBlinkRate 0.5)
    (Utilities|FlowControl|Delay 4.0)
    (CallFunction|SetBlinkRate 0.4)
    (Utilities|FlowControl|Delay 4.0)
    (CallFunction|SetBlinkRate 0.2)
    (Utilities|FlowControl|Delay 3.0)
    (CallFunction|SetBlinkRate 0.08)
    (Utilities|Time|SetTimerbyEvent (delegate Custom|MineExplosion) 3.5) ; Need time to equald 14.5 when adding all previous delays
  ))

(event Custom|MineExplosion
  ;[0.15 0.15 0.15 0.5] Mine Explosion Logic
  (bind _outactors (Collision|SphereOverlapActors (Transformation|GetActorLocation) 3e+02 (Utilities|Array|MakeArray "ObjectTypeQuery3") 0))
  (for _array_element _outactors
    (Class|KismetSystemLibrary|IsObjectOfSoftClass _array_element "/Game/GameAssets/Blueprint/Player/BP_Player.BP_Player_C"
      (:True
        (bind _asbp_player (Utilities|Casting|CastToBP_Player _array_element))
        (if (not (Variables|/Game/GameAssets/Blueprint/Player/BP_Player.BP_Player_C|GetIsDead _asbp_player))
          (Default|Die _asbp_player)
          (bind _asplayer_controller (Utilities|Casting|CastToPlayerController (Pawn|GetController _asbp_player)))
          (bind _asplayer_controller_2 (Utilities|Casting|CastToPlayerController (Game|GetInstigatorController (Components|GetOwner))))
          (bind _asbp_in_game_game_state (Utilities|Casting|CastToBP_InGameGameState (Game|GetGameState)))
          (bind _returnvalue (Class|AdvancedSteamFriendsLibrary|GetSteamPersonaName (Class|AdvancedSessionsLibrary|GetUniqueNetID _asplayer_controller_2)))
          (bind _returnvalue_2 (Class|AdvancedSteamFriendsLibrary|GetSteamPersonaName (Class|AdvancedSessionsLibrary|GetUniqueNetID _asplayer_controller)))
          (Default|AddtoKillfeed _asbp_in_game_game_state (Utilities|Text|ToText(String) (Utilities|String|Append _returnvalue " Killed " _returnvalue_2)))))))
  (Niagara|SpawnSystematLocation "/Game/MixedVFX/Particles/Explosions/NS_ExplosionGroundBig.NS_ExplosionGroundBig" (Transformation|GetActorLocation) "0, 0, 0" "0.500000,0.500000,0.500000")
  (Audio|PlaySoundatLocation "/Game/GameAssets/Assets/SFX/TankDeath.TankDeath" (Transformation|GetActorLocation) "0, 0, 0" 0.1 (Math|Random|RandomFloatinRange 0.9 1.1) 0.0 "/Game/GameAssets/Assets/SFX/SA_Shell.SA_Shell" 0 0 0)
  (Audio|Components|Audio|Stop (Variables|Default|GetBeepingSFX))
  (Actor|DestroyActor))

(event Custom|LightBeep
  (bind _arming_light (Variables|Default|GetArming%20Light))
  ;[0.15 0.15 0.15 0.5] Handle Explosion Beeping
  (Utilities|FlowControl|FlipFlop
    (:A
      (Rendering|SetVisibility _arming_light true false))
    (:B
      (Rendering|SetVisibility _arming_light false false))))

(event Custom|SetBlinkRate
  (params (BlinkInterval :type Float%20%28double-precision%29))
  ;[0.15 0.15 0.15 0.5] Handle Explosion Beeping
  (Utilities|Time|ClearandInvalidateTimerbyHandle (Variables|Default|GetBeepTimer))
  (bind _returnvalue (Utilities|Time|SetTimerbyEvent (delegate Custom|LightBeep) BlinkInterval true))
  (Variables|Default|SetBeepTimer _returnvalue))

(event EventBeginPlay
  (Variables|Default|SetIsActivated false))

(fn ConstructionScript)