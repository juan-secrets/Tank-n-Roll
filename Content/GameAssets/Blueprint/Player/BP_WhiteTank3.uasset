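; BP_WhiteTank3 is a player tank variant with two muzzles that fires mortar-style shells at an impact point.
; SpawnShell alternates muzzles through a FlipFlop, spawning a shell and setting its velocity from a high-arc projectile velocity solve.
; Each shell joins ActiveTankShells and leaves it on destruction, tracking live shells for a limit that is not enforced in this graph.
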(event Custom|CustomEvent_1
  (params (DestroyedActor :type Actor%20Object%20Reference))
  ;[0.15 0.15 0.15 0.5] Limit Active shell to 5
  (bind _asbp_shell (Utilities|Casting|CastToBP_Shell DestroyedActor))
  (Utilities|Array|RemoveItem (Variables|Default|GetActiveTankShells) _asbp_shell))

(event Custom|CustomEvent
  (params (DestroyedActor :type Actor%20Object%20Reference))
  ;[0.15 0.15 0.15 0.5] Limit Active shell to 5
  (bind _asbp_shell (Utilities|Casting|CastToBP_Shell DestroyedActor))
  (Utilities|Array|RemoveItem (Variables|Default|GetActiveTankShells) _asbp_shell))

(event EventBeginPlay
  (|CallParentFunction) ; This node is disabled and will not be called.\nDrag off pins to build functionality.
)

(event Collision|EventActorBeginOverlap
  (params (OtherActor :type Actor%20Object%20Reference)))

(event EventTick
  (params (DeltaSeconds :type Float%20%28single-precision%29))
  (|CallParentFunction DeltaSeconds) ; This node is disabled and will not be called.\nDrag off pins to build functionality.
)

(event EventSpawnShell
  (params (SpawnLocation :type Vector :default "0, 0, 0") (SpawnZRotation :type Float%20%28double-precision%29))
  (Utilities|FlowControl|FlipFlop
    (:A
      ;[0.15 0.15 0.15 0.5] Mortar trajectory
      (bind _returnvalue (Game|SpawnActorfromClass (Variables|Default|GetShellClass) (Math|Transform|MakeTransform (Transformation|GetSocketLocation (Variables|Default|GetMuzzle) "None") (Math|Rotator|MakeRotator 0.0 0.0 0.0) "1.000000,1.000000,1.000000") "Undefined" "MultiplyWithRoot" self 0))
      (Variables|Default|SetSpawnedShell _returnvalue)
      (bind _tossvelocity (Class|GameplayStatics|BlueprintSuggestProjectileVelocity (Transformation|GetSocketLocation (Variables|Default|GetMuzzle) "None") (Variables|Default|GetImpact%20Point) 1.2e+03 0.0 "DoNotTrace" 0.0 true false false))
      (Variables|/Script/Engine.MovementComponent|SetVelocity (Actor|GetComponentbyClass (Variables|Default|GetSpawnedShell) "/Script/Engine.ProjectileMovementComponent") _tossvelocity)
      ;[0.15 0.15 0.15 0.5] Limit Active shell to 5
      (Utilities|Array|AddUnique (Variables|Default|GetActiveTankShells) (Variables|Default|GetSpawnedShell))
      (Game|AssignOnDestroyed (Variables|Default|GetSpawnedShell) (delegate Custom|CustomEvent)))
    (:B
      ;[0.15 0.15 0.15 0.5] Mortar trajectory
      (bind _returnvalue_2 (Game|SpawnActorfromClass (Variables|Default|GetShellClass) (Math|Transform|MakeTransform (Transformation|GetSocketLocation (Variables|Default|GetMuzzle1) "None") (Math|Rotator|MakeRotator 0.0 0.0 0.0) "1.000000,1.000000,1.000000") "Undefined" "MultiplyWithRoot" self 0))
      (Variables|Default|SetSpawnedShell _returnvalue_2)
      (bind _tossvelocity_2 (Class|GameplayStatics|BlueprintSuggestProjectileVelocity (Transformation|GetSocketLocation (Variables|Default|GetMuzzle1) "None") (Variables|Default|GetImpact%20Point) 1.2e+03 0.0 "DoNotTrace" 0.0 true false false))
      (Variables|/Script/Engine.MovementComponent|SetVelocity (Actor|GetComponentbyClass (Variables|Default|GetSpawnedShell) "/Script/Engine.ProjectileMovementComponent") _tossvelocity_2)
      ;[0.15 0.15 0.15 0.5] Limit Active shell to 5
      (Utilities|Array|AddUnique (Variables|Default|GetActiveTankShells) (Variables|Default|GetSpawnedShell))
      (Game|AssignOnDestroyed (Variables|Default|GetSpawnedShell) (delegate Custom|CustomEvent_1)))))

(fn ConstructionScript
  (|CallParentFunction))