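; BP_BlueTank3 is a player tank variant that lobs mortar shells at the point under the mouse cursor.
; MineforAll plays empty-fire audio at the active-shell limit, otherwise fires with sound, camera shake and Niagara effect.
; SpawnMine alternates between two muzzles, using a suggested high-arc projectile velocity to reach the impact point.
; Spawned shells are tracked in ActiveMortar and removed through their OnDestroyed event.
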(event Custom|CustomEvent
  (params (DestroyedActor :type Actor%20Object%20Reference))
  ;[0.15 0.15 0.15 0.5] Limit Active shell to 5
  (bind _asbp_shell (Utilities|Casting|CastToBP_Shell DestroyedActor))
  (Utilities|Array|RemoveItem (Variables|Default|GetActiveMortar) _asbp_shell))

(event EventBeginPlay
  (|CallParentFunction) ; This node is disabled and will not be called.\nDrag off pins to build functionality.
)

(event Collision|EventActorBeginOverlap
  (params (OtherActor :type Actor%20Object%20Reference)))

(event EventTick
  (params (DeltaSeconds :type Float%20%28single-precision%29))
  (|CallParentFunction DeltaSeconds))

(event EventMineforAll
  (if (>= (Utilities|Array|Length (Variables|Default|GetActiveMortar)) (Variables|Default|GetMineLimit))
    (Audio|PlaySoundatLocation "/Game/GameAssets/Assets/SFX/EmptyFire.EmptyFire" (Transformation|GetActorLocation) "0, 0, 0" 0.1 (Math|Random|RandomFloatinRange 0.9 1.1) 0.0 "/Game/GameAssets/Assets/SFX/SA_Shell.SA_Shell" 0 0 0)
    (else
      (Audio|PlaySoundatLocation "/Game/GameAssets/Assets/SFX/TankShot.TankShot" (Transformation|GetActorLocation) "0, 0, 0" 0.1 (Math|Random|RandomFloatinRange 0.9 1.1) 0.0 "/Game/GameAssets/Assets/SFX/SA_Shell.SA_Shell" 0 0 0)
      (CameraShakes|StartCameraShake (Game|GetPlayerCameraManager 0) "/Game/GameAssets/Blueprint/Player/CS_TankShoot.CS_TankShoot_C" 1.0 "CameraLocal" "0, 0, 0")
      (CallFunction|SpawnMine "0, 0, 0" (.ImpactPoint (Collision|BreakHitResult (.HitResult (Game|Player|GetHitResultUnderCursorbyChannel (Game|GetPlayerController 0) "TraceTypeQuery1" true)))))
      (Niagara|SpawnSystematLocation "/Game/MixedVFX/Particles/Projectiles/Hits/NS_FireArrow_Hit.NS_FireArrow_Hit" (Transformation|GetSocketLocation (Variables|Default|GetMuzzle) "None")))))

(event EventSpawnMine
  (params (SpawnLocation :type Vector :default "0, 0, 0") (ImpactPoint :type Vector :default "0, 0, 0"))
  (Utilities|FlowControl|FlipFlop
    (:A
      ;[0.15 0.15 0.15 0.5] Mortar trajectory
      (bind _returnvalue (Game|SpawnActorfromClass "/Game/GameAssets/Blueprint/Props/BP_MortarShell.BP_MortarShell_C" (Math|Transform|MakeTransform (Transformation|GetSocketLocation (Variables|Default|GetMuzzle1) "None") (Math|Rotator|MakeRotator 0.0 0.0 0.0) "1.000000,1.000000,1.000000") "Undefined" "MultiplyWithRoot" self 0))
      (Variables|Default|SetSpawnedShell _returnvalue)
      (bind _tossvelocity (Class|GameplayStatics|BlueprintSuggestProjectileVelocity (Transformation|GetSocketLocation (Variables|Default|GetMuzzle1) "None") ImpactPoint 1.2e+03 0.0 "DoNotTrace" 0.0 true false false))
      (Variables|/Script/Engine.MovementComponent|SetVelocity (Actor|GetComponentbyClass (Variables|Default|GetSpawnedShell) "/Script/Engine.ProjectileMovementComponent") _tossvelocity)
      ;[0.15 0.15 0.15 0.5] Limit Active shell to 5
      (Utilities|Array|AddUnique (Variables|Default|GetActiveMortar) (Variables|Default|GetSpawnedShell))
      (Game|AssignOnDestroyed (Variables|Default|GetSpawnedShell) (delegate Custom|CustomEvent)))
    (:B
      ;[0.15 0.15 0.15 0.5] Mortar trajectory
      (bind _returnvalue_2 (Game|SpawnActorfromClass "/Game/GameAssets/Blueprint/Props/BP_MortarShell.BP_MortarShell_C" (Math|Transform|MakeTransform (Transformation|GetSocketLocation (Variables|Default|GetMuzzle2) "None") (Math|Rotator|MakeRotator 0.0 0.0 0.0) "1.000000,1.000000,1.000000") "Undefined" "MultiplyWithRoot" self 0))
      (Variables|Default|SetSpawnedShell _returnvalue_2)
      (bind _tossvelocity_2 (Class|GameplayStatics|BlueprintSuggestProjectileVelocity (Transformation|GetSocketLocation (Variables|Default|GetMuzzle2) "None") ImpactPoint 1.2e+03 0.0 "DoNotTrace" 0.0 true false false))
      (Variables|/Script/Engine.MovementComponent|SetVelocity (Actor|GetComponentbyClass (Variables|Default|GetSpawnedShell) "/Script/Engine.ProjectileMovementComponent") _tossvelocity_2)
      ;[0.15 0.15 0.15 0.5] Limit Active shell to 5
      (Utilities|Array|AddUnique (Variables|Default|GetActiveMortar) (Variables|Default|GetSpawnedShell))
      (Game|AssignOnDestroyed (Variables|Default|GetSpawnedShell) (delegate Custom|CustomEvent)))))

(fn ConstructionScript
  (|CallParentFunction))