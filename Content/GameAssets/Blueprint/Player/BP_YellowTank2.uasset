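; Yellow tank variant Blueprint that fires shells from two alternating muzzle positions.
; SpawnShell uses a FlipFlop to spawn the shell class at either the passed-in location or the Muzzle1 component, sharing the same yaw.
; Each shell is added to ActiveTankShells and removed when destroyed, tracking live shells for an active-shell limit that is not enforced in this graph.
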(event Custom|CustomEvent
  (params (DestroyedActor :type Actor%20Object%20Reference))
  ;[0.15 0.15 0.15 0.5] Limit Active shell to 5
  (bind _asbp_shell (Utilities|Casting|CastToBP_Shell DestroyedActor))
  (Utilities|Array|RemoveItem (Variables|Default|GetActiveTankShells) _asbp_shell))

(event EventBeginPlay
  (|CallParentFunction) ; This node is disabled and will not be called.\nDrag off pins to build functionality.
)

(event Collision|EventActorBeginOverlap
  (params (OtherActor :type Actor%20Object%20Reference)))

(event EventTick
  (params (DeltaSeconds :type Float%20%28single-precision%29))
  (|CallParentFunction DeltaSeconds) ; This node is disabled and will not be called.\nDrag off pins to build functionality.
)

(event EventSpawnShell
  (params (SpawnLocation :type Vector :default "0, 0, 0") (SpawnZRotation :type Float%20%28double-precision%29))
  (Utilities|FlowControl|FlipFlop
    (:A
      ;[0.15 0.15 0.15 0.5] Spawn PrimaryFire Shell
      (bind _returnvalue (Game|SpawnActorfromClass (Variables|Default|GetShellClass) (Math|Transform|MakeTransform SpawnLocation (Math|Rotator|MakeRotator 0.0 0.0 SpawnZRotation) "1.000000,1.000000,1.000000") "Undefined" "MultiplyWithRoot" self 0))
      ;[0.15 0.15 0.15 0.5] Limit Active shell to 5
      (Utilities|Array|AddUnique (Variables|Default|GetActiveTankShells) _returnvalue)
      (Game|AssignOnDestroyed _returnvalue (delegate Custom|CustomEvent)))
    (:B
      ;[0.15 0.15 0.15 0.5] Spawn PrimaryFire Shell
      (bind _returnvalue_2 (Game|SpawnActorfromClass (Variables|Default|GetShellClass) (Math|Transform|MakeTransform (Transformation|GetWorldLocation (Variables|Default|GetMuzzle1)) (Math|Rotator|MakeRotator 0.0 0.0 SpawnZRotation) "1.000000,1.000000,1.000000") "Undefined" "MultiplyWithRoot" self 0))
      ;[0.15 0.15 0.15 0.5] Limit Active shell to 5
      (Utilities|Array|AddUnique (Variables|Default|GetActiveTankShells) _returnvalue_2)
      (Game|AssignOnDestroyed _returnvalue_2 (delegate Custom|CustomEvent)))))

(fn ConstructionScript
  (|CallParentFunction))