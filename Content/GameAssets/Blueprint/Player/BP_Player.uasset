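; Player-controlled tank character for multiplayer, handling movement, cursor aiming, shooting, death and win/lose screens.
; Tick drives the body from Enhanced Input, turns the cannon toward the cursor hit through a server event and feeds speed to engine audio.
; While moving, a looping timer spawns server-side track marks; firing caps live shells at five via OnDestroyed tracking.
; Death sets IsDead, whose OnRep notifies BP_GameplayMode on authority; destruction cleans up effects, shells and widgets.
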(event Custom|Server_DrawTrackTrace
  ;[0.15 0.15 0.15 0.5] Spawn Tank Black Traces
  (if (< (Variables|Default|GetMoveValueY) 0.0)
    (Game|SpawnActorfromClass "/Game/GameAssets/Blueprint/Player/BP_TankTrace.BP_TankTrace_C" (Math|Transform|MakeTransform (Transformation|GetWorldLocation (Variables|Default|GetR_TrackFront)) (Transformation|GetActorRotation)) "Undefined" "MultiplyWithRoot" 0 0)
    (Game|SpawnActorfromClass "/Game/GameAssets/Blueprint/Player/BP_TankTrace.BP_TankTrace_C" (Math|Transform|MakeTransform (Transformation|GetWorldLocation (Variables|Default|GetL_TrackFront)) (Transformation|GetActorRotation)) "Undefined" "MultiplyWithRoot" 0 0)
    (else
      (Game|SpawnActorfromClass "/Game/GameAssets/Blueprint/Player/BP_TankTrace.BP_TankTrace_C" (Math|Transform|MakeTransform (Transformation|GetWorldLocation (Variables|Default|GetR_TrackBack)) (Transformation|GetActorRotation)) "Undefined" "MultiplyWithRoot" 0 0)
      (Game|SpawnActorfromClass "/Game/GameAssets/Blueprint/Player/BP_TankTrace.BP_TankTrace_C" (Math|Transform|MakeTransform (Transformation|GetWorldLocation (Variables|Default|GetL_TrackBack)) (Transformation|GetActorRotation)) "Undefined" "MultiplyWithRoot" 0 0))))

(event Custom|DrawTrackTrace
  ;[0.15 0.15 0.15 0.5] Player Move
  (CallFunction|ServerDrawTrackTrace))

(event Custom|Server_SetCannonRotation
  (params (Z%20Rotation :type Float%20%28double-precision%29))
  ;[0.15 0.15 0.15 0.5] Set Cannon Rotation Based on Mouse World Position
  (Transformation|SetWorldRotation (Variables|Default|GetSM_TankCannon) (Math|Rotator|MakeRotator 0.0 0.0 Z%20Rotation) false false))

(event Custom|Client_SetCannonRotation
  ;[0.15 0.15 0.15 0.5] Set Cannon Rotation Based on Mouse World Position
  (CallFunction|ServerSetCannonRotation (Math|Rotator|NormalizeAxis (+ (.yaw (Math|Rotator|FindLookatRotation (Transformation|GetActorLocation) (.ImpactPoint (Collision|BreakHitResult (.HitResult (Game|Player|GetHitResultUnderCursorbyChannel (Game|GetPlayerController 0) "TraceTypeQuery1" true)))))) -9e+01))))

(event Input|EnhancedActionEvents|EnhancedInputActionIA_PlayerMove
  (params (ActionValue :type Vector%202D%20Structure) (ElapsedSeconds :type Float%20%28double-precision%29) (TriggeredSeconds :type Float%20%28double-precision%29) (InputAction :type Input%20Action%20Object%20Reference :default "/Game/GameAssets/Blueprint/Player/Controls/IA_PlayerMove.IA_PlayerMove"))
  ;[0.15 0.15 0.15 0.5] Player Move
  (:Triggered
    (Variables|Default|SetMoveValueX (.x ActionValue))
    (Variables|Default|SetMoveValueY (.y ActionValue))
    (Variables|Default|SetIsMoving true)
    (if (not (Utilities|Time|IsValidTimerHandle (Variables|Default|GetTrackGroundTraceHandle)))
      (bind _returnvalue (Utilities|Time|SetTimerbyEvent (delegate Custom|DrawTrackTrace) (Variables|Default|GetTimeBetweenTraces) true))
      (Variables|Default|SetTrackGroundTraceHandle _returnvalue)))
  (:Completed
    (Variables|Default|SetIsMoving false)
    (Utilities|Time|ClearandInvalidateTimerbyHandle (Variables|Default|GetTrackGroundTraceHandle))))

(event EventBeginPlay
  ;[0.15 0.15 0.15 0.5] Setup IMC
  (Utilities|FlowControl|DelayUntilNextTick)
  (Input|AddMappingContext (PlayerController|LocalPlayerSubsystems|GetEnhancedInputLocalPlayerSubsystem (Game|GetPlayerController 0)) "/Game/GameAssets/Blueprint/Player/Controls/IMC_Player.IMC_Player" 0 "(bIgnoreAllPressedKeysUntilRelease=True,bForceImmediately=False,bNotifyUserSettings=False)")
  ;[0.15 0.15 0.15 0.5] Set reticule
  (if (Pawn|IsLocallyControlled)
    (bind _returnvalue (UserInterface|CreateWidget "/Game/GameAssets/Blueprint/UI/WBP_AimReticule.WBP_AimReticule_C"))
    (bind _output_get (Variables|Default|SetReticuleWidget _returnvalue))
    (UserInterface|Viewport|AddtoViewport _output_get 0)
    (Variables|/Script/Engine.PlayerController|SetbShowMouseCursor (Game|GetPlayerController 0) false)))

(event EventTick
  (params (DeltaSeconds :type Float%20%28single-precision%29))
  (bind _returnvalue (Transformation|GetActorRotation))
  ;[0.15 0.15 0.15 0.5] Event Tick
  (Utilities|FlowControl|Sequence
    (:then_0
      ;;[0.15 0.15 0.15 0.5] Tank Body Movements
      (if (Variables|Default|GetIsMoving)
        (Pawn|Input|AddMovementInput (Transformation|GetActorForwardVector) (Variables|Default|GetMoveValueY) false)
        (Pawn|SetControlRotation (Pawn|GetController) (Math|Rotator|MakeRotator (.roll _returnvalue) (.pitch _returnvalue) (Math|Rotator|NormalizeAxis (+ (.yaw _returnvalue) (* (Variables|Default|GetMoveValueX) (* (Variables|Default|GetBodyRotationSpeed) DeltaSeconds))))))))
    (:then_1
      ;;[0.15 0.15 0.15 0.5] Tank Cannon Rotation
      (CallFunction|ClientSetCannonRotation))
    (:then_2
      ;;[0.15 0.15 0.15 0.5] Set Speed for engine SFX
      (Audio|Parameter|SetFloatParameter (Variables|Default|GetTankEngine) "None" (Math|Vector|VectorLength (Transformation|GetVelocity)) :!class /Script/Engine.AudioComponent))))

(event Custom|FireForAll
  (bind _muzzle (Variables|Default|GetMuzzle))
  (bind _returnvalue (Transformation|GetWorldLocation _muzzle))
  ;[0.15 0.15 0.15 0.5] Run on Server: Create shell
  (if (> (Utilities|Array|Length (Variables|Default|GetActiveTankShells)) 4)
    (Audio|PlaySoundatLocation "/Game/GameAssets/Assets/SFX/EmptyFire.EmptyFire" (Transformation|GetActorLocation) "0, 0, 0" 0.1 (Math|Random|RandomFloatinRange 0.9 1.1) 0.0 "/Game/GameAssets/Assets/SFX/SA_Shell.SA_Shell" 0 0 0)
    (else
      (Audio|PlaySoundatLocation "/Game/GameAssets/Assets/SFX/TankShot.TankShot" (Transformation|GetActorLocation) "0, 0, 0" 0.1 (Math|Random|RandomFloatinRange 0.9 1.1) 0.0 "/Game/GameAssets/Assets/SFX/SA_Shell.SA_Shell" 0 0 0)
      (CameraShakes|StartCameraShake (Game|GetPlayerCameraManager 0) "/Game/GameAssets/Blueprint/Player/CS_TankShoot.CS_TankShoot_C" 1.0 "CameraLocal" "0, 0, 0")
      (CallFunction|SpawnShell _returnvalue (.yaw (Math|Rotator|FindLookatRotation _returnvalue (.ImpactPoint (Collision|BreakHitResult (.HitResult (Game|Player|GetHitResultUnderCursorbyChannel (Game|GetPlayerController 0) "TraceTypeQuery1" true)))))))
      (Niagara|SpawnSystematLocation "/Game/MixedVFX/Particles/Projectiles/Hits/NS_FireArrow_Hit.NS_FireArrow_Hit" (Transformation|GetSocketLocation (Variables|Default|GetMuzzle) "None")))))

(event Custom|OnDestroyed_Event
  (params (DestroyedActor :type Actor%20Object%20Reference))
  ;[0.15 0.15 0.15 0.5] Limit Active shell to 5
  (bind _asbp_shell (Utilities|Casting|CastToBP_Shell DestroyedActor))
  (Utilities|Array|RemoveItem (Variables|Default|GetActiveTankShells) _asbp_shell))

(event Custom|SpawnShell
  (params (SpawnLocation :type Vector) (SpawnZRotation :type Float%20%28double-precision%29))
  (bind _returnvalue (Game|SpawnActorfromClass "/Game/GameAssets/Blueprint/Props/BP_Shell.BP_Shell_C" (Math|Transform|MakeTransform SpawnLocation (Math|Rotator|MakeRotator 0.0 0.0 SpawnZRotation) "1.000000,1.000000,1.000000") "Undefined" "MultiplyWithRoot" self 0))
  ;[0.15 0.15 0.15 0.5] Limit Active shell to 5
  (Utilities|Array|AddUnique (Variables|Default|GetActiveTankShells) _returnvalue)
  (Game|AssignOnDestroyed _returnvalue (delegate Custom|OnDestroyed_Event)))

(event Input|EnhancedActionEvents|EnhancedInputActionIA_Shoot
  (params (ActionValue :type Boolean) (ElapsedSeconds :type Float%20%28double-precision%29) (TriggeredSeconds :type Float%20%28double-precision%29) (InputAction :type Input%20Action%20Object%20Reference :default "/Game/GameAssets/Blueprint/Player/Controls/IA_Shoot.IA_Shoot"))
  ;[0.15 0.15 0.15 0.5] Fire Input
  (:Started
    (if (not (Variables|Default|GetIsDead))
      (CallFunction|FireforAll))))

(event Custom|LostGame
  ;[0.15 0.15 0.15 0.5] Win / Lose
  (bind _asplayer_controller (Utilities|Casting|CastToPlayerController (Pawn|GetController)))
  (Input|SetInputModeUIOnly _asplayer_controller 0 "DoNotLock" false)
  (bind _returnvalue (UserInterface|CreateWidget "/Game/GameAssets/Blueprint/UI/Menus/WinLose/WBP_LostGame.WBP_LostGame_C"))
  (Variables|Default|SetEndGameWidget _returnvalue)
  (UserInterface|Viewport|AddtoViewport _returnvalue 0))

(event Custom|WonGame
  ;[0.15 0.15 0.15 0.5] Win / Lose
  (bind _asplayer_controller (Utilities|Casting|CastToPlayerController (Pawn|GetController)))
  (Input|SetInputModeUIOnly _asplayer_controller 0 "DoNotLock" false)
  (bind _returnvalue (UserInterface|CreateWidget "/Game/GameAssets/Blueprint/UI/Menus/WinLose/WBP_WinGame.WBP_WinGame_C"))
  (Variables|Default|SetEndGameWidget _returnvalue)
  (UserInterface|Viewport|AddtoViewport _returnvalue 0))

(event Custom|MainMenu
  ;[0.15 0.15 0.15 0.5] Win / Lose
  (Development|PrintString "in main menu function" true true "(R=1.000000,G=0.901120,B=0.974491,A=1.000000)" 1e+04)
  (if (Ability|HasAuthority (Game|GetPlayerController 0))
    (Utilities|FlowControl|Delay 0.5)
    (else
      (Utilities|FlowControl|Delay 0.25)))
  (Game|OpenLevel(byName) "MainMenu"))

(event Custom|Die
  (bind _returnvalue (Math|Random|RandomFloatinRange 0.8 1.2))
  (bind _returnvalue_2 (Transformation|GetActorLocation))
  ;[0.15 0.15 0.15 0.5] Die Event
  (Variables|Default|SetIsDead true)
  (Pawn|Components|CharacterMovement|DisableMovement (Variables|Character|GetCharacterMovement))
  (Audio|PlaySoundatLocation "/Game/GameAssets/Assets/SFX/TankDeath.TankDeath" (Transformation|GetActorLocation) "0, 0, 0" 0.1 (Math|Random|RandomFloatinRange 0.9 1.1) 0.0 "/Game/GameAssets/Assets/SFX/SA_Shell.SA_Shell" 0 0 0)
  (Audio|Components|Audio|FadeOut (Variables|Default|GetTankEngine) 0.5 0.0 "Linear" :!class /Script/Engine.AudioComponent)
  (bind _returnvalue_3 (Niagara|SpawnSystematLocation "/Game/MixedVFX/Particles/Explosions/NS_ExplosionGroundSmall.NS_ExplosionGroundSmall" _returnvalue_2 (Math|Random|RandomRotator true) (Math|Vector|MakeVector _returnvalue _returnvalue _returnvalue)))
  (bind _returnvalue_4 (Niagara|SpawnSystematLocation "/Game/MixedVFX/Particles/Mix/NS_Mix_02.NS_Mix_02" _returnvalue_2 "0, 0, 0" (Math|Vector|MakeVector _returnvalue _returnvalue _returnvalue)))
  (Utilities|Array|Add (Variables|Default|GetNiagaraSystems) _returnvalue_4)
  (Utilities|Array|Add (Variables|Default|GetNiagaraSystems) _returnvalue_3))

(event Custom|Destroy
  ;[0.15 0.15 0.15 0.5] Destroy Event - Clean residual niagara effects, shells and widgets
  (Utilities|FlowControl|Sequence
    (:then_0
      (for _array_element (Variables|Default|GetNiagaraSystems)
        (Utilities|IsValid _array_element
          (:Is%20Valid
            (Components|DestroyComponent _array_element)))))
    (:then_1
      (for _array_element_2 (Variables|Default|GetActiveTankShells)
        (Utilities|IsValid _array_element_2
          (:Is%20Valid
            (Actor|DestroyActor _array_element_2)))))
    (:then_2
      (Utilities|IsValid (Variables|Default|GetEndGameWidget)
        (:Is%20Valid
          (Widget|RemovefromParent (Variables|Default|GetEndGameWidget))
          (Input|SetInputModeGameOnly (Game|GetPlayerController 0) false))))
    (:then_3
      (Actor|DestroyActor))))

(event EventDestroyed
  ;[0.15 0.15 0.15 0.5] Destroy Event - Clean residual niagara effects, shells and widgets
  (CallFunction|Destroy))

(fn ConstructionScript)

(fn OnRepIsDead
  (if (and (Variables|Default|GetIsDead) (Ability|HasAuthority))
    (bind _asbp_gameplay_mode (Utilities|Casting|CastToBP_GameplayMode (Game|GetGameMode))
      (:then
        (bind _asplayer_controller (Utilities|Casting|CastToPlayerController (Pawn|GetController))
          (:then
            (Default|PlayerDied _asbp_gameplay_mode _asplayer_controller))
          (:CastFailed
            (Development|PrintString "Cast to PlayerController failed in BP_Player"))))
      (:CastFailed
        (Development|PrintString "Cast to BP_GameplayMode failed in BP_Player")))))