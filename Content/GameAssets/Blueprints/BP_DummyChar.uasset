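; BP_DummyChar is a bare-bones test character driven by debug keys, with a way to leave a multiplayer session.
; Z/Q/S/D latch a world direction from the capsule's forward and right vectors, and E clears it.
; Tick applies that direction as forced movement input, so movement continues after key release.
; A destroys the session and loads MainMenu on success; BeginPlay sets game-only input with a visible cursor.
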(event EventBeginPlay
  (bind _returnvalue (Game|GetPlayerController 0))
  (Input|SetInputModeGameOnly _returnvalue false)
  (Development|PrintString "Set input mode game only")
  (Variables|/Script/Engine.PlayerController|SetbShowMouseCursor _returnvalue true))

(event EventTick
  (params (DeltaSeconds :type Float%20%28single-precision%29))
  (Pawn|Input|AddMovementInput (Class|PawnMovementComponent|GetPawnOwner (Variables|Character|GetCharacterMovement)) (* (Variables|Default|GetWorld%20Direction) (Math|Float|MakeLiteralFloat 1.0)) 1.0 true))

(event Input|KeyboardEvents|DebugKeyD
  (params (Key :type Key%20Structure :default "None") (ActionValue :type Input%20Action%20Value%20Structure))
  (:Pressed
    (Variables|Default|SetWorld%20Direction (Math|Vector|GetRightVector (Variables|Collision|GetCapsuleComponent)))))

(event Input|KeyboardEvents|DebugKeyA
  (params (Key :type Key%20Structure :default "None") (ActionValue :type Input%20Action%20Value%20Structure))
  (:Pressed
    (|DestroySession (Game|GetPlayerController 0)
      (:OnSuccess
        (Utilities|FlowControl|Delay 0.25)
        (Game|OpenLevel(byName) "MainMenu"))
      (:OnFailure
        (Development|PrintString "Failed to leave the session")))))

(event Input|KeyboardEvents|DebugKeyE
  (params (Key :type Key%20Structure :default "None") (ActionValue :type Input%20Action%20Value%20Structure))
  (:Pressed
    (Variables|Default|SetWorld%20Direction "0, 0, 0")))

(event Input|KeyboardEvents|DebugKeyZ
  (params (Key :type Key%20Structure :default "None") (ActionValue :type Input%20Action%20Value%20Structure))
  (:Pressed
    (Variables|Default|SetWorld%20Direction (Math|Vector|GetForwardVector (Variables|Collision|GetCapsuleComponent)))))

(event Input|KeyboardEvents|DebugKeyQ
  (params (Key :type Key%20Structure :default "None") (ActionValue :type Input%20Action%20Value%20Structure))
  (:Pressed
    (Variables|Default|SetWorld%20Direction (* (Math|Vector|GetRightVector (Variables|Collision|GetCapsuleComponent)) (Math|Float|MakeLiteralFloat -1.0)))))

(event Input|KeyboardEvents|DebugKeyS
  (params (Key :type Key%20Structure :default "None") (ActionValue :type Input%20Action%20Value%20Structure))
  (:Pressed
    (Variables|Default|SetWorld%20Direction (* (Math|Vector|GetForwardVector (Variables|Collision|GetCapsuleComponent)) (Math|Float|MakeLiteralFloat -1.0)))))

(fn ConstructionScript)